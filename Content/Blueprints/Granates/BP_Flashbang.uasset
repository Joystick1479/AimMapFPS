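; BP_Flashbang is a thrown flashbang grenade that launches itself on BeginPlay and detonates after three seconds.
; BeginPlay calls the throw event once per BP_SoldierCharacter, each call playing the pin sound and adding forward and random spin impulses.
; Detonation spawns a decal, passes distance and grenade location to every soldier's Flashbang, and calls DestroyActor inside that loop.
; Pin and explosion sounds route through multicast-named events with attenuation.
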(event `ThrowinGranade`
  (params (Impulse :type "Vector Structure") (Impulse2 :type "Vector Structure") (Target :type "/Game/Blueprints/BP_SoldierCharacter Object Reference"))
  (bind _returnvalue (`self.K2_GetActorLocation`))
  (bind _staticmesh (`self.StaticMesh`))
  (`self.PinPullSound`)
  (`PrimitiveComponent.AddImpulse` _staticmesh Impulse "None" true)
  (`PrimitiveComponent.AddAngularImpulseInDegrees` _staticmesh Impulse2 "None" true)
  (`KismetSystemLibrary.Delay` 3.0)
  (`self.ExplosionSound`)
  (`|SpawnActorFromClass` "/Game/Blueprints/Granates/BP_ExplosionDecal.BP_ExplosionDecal_C" (`KismetMathLibrary.MakeTransform` _returnvalue (struct :`Pitch` 90.0)) "Undefined" "OverrideRootScale" null null)
  (bind _outactors (`GameplayStatics.GetAllActorsOfClass` "/Game/Blueprints/BP_SoldierCharacter.BP_SoldierCharacter_C"))
  (for _array_element _outactors
    (`/Game/Blueprints/BP_SoldierCharacter.Flashbang` _array_element (`self.GetDistanceTo` _array_element) _returnvalue)
    (`self.K2_DestroyActor`)))

(event `ExplosionSound`
  ;[1 1 1] Explosion sound
  (`self.ExplosionSoundMulticast`))

(event `ExplosionSoundMulticast`
  ;[1 1 1] Explosion sound
  (`GameplayStatics.SpawnSoundAtLocation` "/Game/Audio/Grenade/GrenadeSound_Cue.GrenadeSound_Cue" (`self.K2_GetActorLocation`) (struct) 2.0 1.0 0.0 "/Game/Audio/Grenade/GrenadeAttentuation.GrenadeAttentuation" null))

(event `self.ReceiveBeginPlay`
  (bind _outactors (`GameplayStatics.GetAllActorsOfClass` "/Game/Blueprints/BP_SoldierCharacter.BP_SoldierCharacter_C"))
  (for _array_element _outactors
    (`self.ThrowinGranade` (* (`SceneComponent.GetForwardVector` (`self.StaticMesh`)) 750.0) (* (`KismetMathLibrary.RandomUnitVector`) 500.0) _array_element)))

(event `PinPullSound`
  ;[1 1 1] PinPullSound
  (`self.PinPulLSoundMulticast`))

(event `PinPulLSoundMulticast`
  ;[1 1 1] PinPullSound
  (`GameplayStatics.SpawnSoundAtLocation` "/Game/Audio/Grenade/hand_grenade_pin_pull_001_Cue.hand_grenade_pin_pull_001_Cue" (`self.K2_GetActorLocation`) (struct) 2.0 1.0 0.0 "/Game/Audio/Grenade/GrenadeAttentuation.GrenadeAttentuation" null))

(fn `UserConstructionScript`)