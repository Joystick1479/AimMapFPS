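; BP_Test is a test payload character that travels toward a BP_BlueTarget when a soldier overlaps it.
; On overlap begin with a BP_SoldierCharacter, its controller runs SimpleMoveToLocation to the first BP_BlueTarget found in the level.
; On overlap end with a soldier, it stops active movement, without counting any soldiers still overlapping.
; A duplicate move-to-target chain is left unconnected.
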(event `self.ReceiveActorBeginOverlap`
  (params (OtherActor :type "Actor Object Reference"))
  (cast `/Game/Blueprints/BP_SoldierCharacter` OtherActor)
  (bind _outactors (`GameplayStatics.GetAllActorsOfClass` "/Game/Blueprints/Payload/BP_BlueTarget.BP_BlueTarget_C"))
  (`AIBlueprintHelperLibrary.SimpleMoveToLocation` (`self.GetController`) (`self.K2_GetActorLocation` (`|GetArrayItem` _outactors))))

(event `self.ReceiveActorEndOverlap`
  (params (OtherActor :type "Actor Object Reference"))
  (cast `/Game/Blueprints/BP_SoldierCharacter` OtherActor)
  (`NavMovementComponent.StopActiveMovement` (`self.CharacterMovement`)))

(event `self.ReceiveTick`
  (params (DeltaSeconds :type "Float (single-precision)")))

(fn `UserConstructionScript`)