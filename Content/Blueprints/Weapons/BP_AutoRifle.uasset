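; Automatic rifle weapon Blueprint that measures how close its soldier owner is to obstacles and provides weapon sway.
; Each Tick, a debug-drawn trace forward from the owning BP_SoldierCharacter sets a clamped DistanceToObject ratio and prints it, identically in both branches.
; WeaponSway eases the skeletal mesh's pitch by a given direction within a small clamped range.
; A muzzle-socket trace variant and rotation tests are left unconnected, and nothing here consumes DistanceToObject.
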(event `self.ReceiveTick`
  (params (DeltaSeconds :type "Float (single-precision)"))
  (bind _asbp_soldier_character (cast `/Game/Blueprints/BP_SoldierCharacter` (`self.GetOwner`)))
  (bind _returnvalue (`self.K2_GetActorLocation` _asbp_soldier_character))
  (bind _outhit (`KismetSystemLibrary.LineTraceSingle` _returnvalue (+ _returnvalue (* (`KismetMathLibrary.GetForwardVector` (`self.K2_GetActorRotation` _asbp_soldier_character)) 150.0)) "TraceTypeQuery1" false (`|MakeArray` (`self.GetOwner`)) "ForOneFrame" true (struct :`R` 1.0 :`A` 1.0) (struct :`G` 1.0 :`A` 1.0) 1.0))
  (bind (_bblockinghit _binitialoverlap _time _distance) (`GameplayStatics.BreakHitResult` _outhit))
  (if (and (< _distance 75.0) (> _distance 0.0))
    (bind _returnvalue_2 (`KismetMathLibrary.FClamp` (/ 75.0 _distance)))
    (bind _output_get (set `self.DistanceToObject` _returnvalue_2))
    (`KismetSystemLibrary.PrintString` (`KismetStringLibrary.Conv_DoubleToString` _output_get))
    (else
      (bind _output_get_2 (set `self.DistanceToObject` _returnvalue_2))
      (`KismetSystemLibrary.PrintString` (`KismetStringLibrary.Conv_DoubleToString` _output_get_2)))))

(fn `UserConstructionScript`)

(fn `WeaponSway`
  (params (SwayDirection :type "Float (double-precision)"))
  (bind _returnvalue (`SceneComponent.GetRelativeTransform` (`self.SkelMeshComp`)))
  (`SceneComponent.K2_SetRelativeRotation` (`self.SkelMeshComp`) (`KismetMathLibrary.RInterpTo` (`KismetMathLibrary.MakeRotator` (.roll (.rotation _returnvalue)) (.pitch (.rotation _returnvalue)) (.yaw (.rotation _returnvalue))) (`KismetMathLibrary.MakeRotator` (.roll (.rotation _returnvalue)) (`KismetMathLibrary.FClamp` (+ (.pitch (.rotation _returnvalue)) SwayDirection) -5.0 5.0) (.yaw (.rotation _returnvalue))) (`GameplayStatics.GetWorldDeltaSeconds`) 3.0) false false))