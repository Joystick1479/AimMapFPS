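; Player character Blueprint that adds hold-to-sprint and hold-to-aim input.
; Left Shift doubles walk speed and sets IsSprinting while held.
; Right mouse sets IsAiming and cubic-blends the view to the first BP_AutomaticRifle in the level, then back to the first BP_MainCharacter on release, both found with GetAllActorsOfClass.
; A rifle cast, a timeline and a head-socket lookup are left unconnected.
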(event `Key|LeftShift`
  (params (Key :type "Key Structure"))
  (bind _charactermovement (`self.CharacterMovement`))
  (:`Pressed`
    (set `CharacterMovementComponent.MaxWalkSpeed` 270.0 _charactermovement)
    (set `self.isSprinting?` true))
  (:`Released`
    (set `CharacterMovementComponent.MaxWalkSpeed` 135.0 _charactermovement)
    (set `self.isSprinting?` false)))

(event `Key|RightMouseButton`
  (params (Key :type "Key Structure"))
  (:`Pressed`
    (set `self.isAiming?` true)
    (bind _asplayer_controller (cast `PlayerController` (`GameplayStatics.GetPlayerController` 0)))
    (bind _outactors (`GameplayStatics.GetAllActorsOfClass` "/Game/Blueprints/Weapons/BP_AutomaticRifle.BP_AutomaticRifle_C"))
    (`PlayerController.SetViewTargetWithBlend` _asplayer_controller (`|GetArrayItem` _outactors) 0.5 "VTBlend_Cubic" 0.0 false))
  (:`Released`
    (set `self.isAiming?` false)
    (bind _outactors_2 (`GameplayStatics.GetAllActorsOfClass` "BP_MainCharacter_C"))
    (`PlayerController.SetViewTargetWithBlend` (`GameplayStatics.GetPlayerController` 0) (`|GetArrayItem` _outactors_2) 0.5 "VTBlend_Cubic" 0.0 false)))

(fn `UserConstructionScript`)