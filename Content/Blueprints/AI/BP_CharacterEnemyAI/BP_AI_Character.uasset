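; BP_AI_Character is an enemy AI character that runs the BT_AdvancedAI behavior tree.
; On BeginPlay it spawns a BP_AI_Weapon, attaches it to the mesh's WeaponSocket and stores it as CurrentWeapon.
; Tick polls the Died flag and, once, destroys the character after a delay, then enables weapon physics.
; A second delay precedes the weapon's destruction, though it is scheduled after the character's own DestroyActor call.
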(event `self.ReceiveBeginPlay`
  (`parent.ReceiveBeginPlay`)
  (`AIController.RunBehaviorTree` (`AIBlueprintHelperLibrary.GetAIController` self) "/Game/Blueprints/AI/BP_CharacterEnemyAI/BT_AdvancedAI.BT_AdvancedAI")
  (bind _returnvalue (`|SpawnActorFromClass` "/Game/Blueprints/AI/BP_CharacterEnemyAI/BP_AI_Weapon.BP_AI_Weapon_C" (`KismetMathLibrary.MakeTransform` (0.0 0.0 0.0)) "AlwaysSpawn" "OverrideRootScale" self null))
  (`self.K2_AttachToComponent` _returnvalue (`self.Mesh`) "WeaponSocket" "SnapToTarget" "SnapToTarget" "SnapToTarget" true)
  (set `self.CurrentWeapon` _returnvalue)
  (set `self.bIsWeaponAttached` true))

(event `self.ReceiveTick`
  (params (DeltaSeconds :type "Float (single-precision)"))
  (bind _currentweapon (`self.CurrentWeapon`))
  (bind _skelmeshcomp (`BaseWeaponClass.SkelMeshComp` _currentweapon))
  (if (`self.bDied`)
    (`/Engine/EditorBlueprintResources/StandardMacros.DoOnce` false
      (:`Completed`
        (`KismetSystemLibrary.Delay` 2.0)
        (`self.K2_DestroyActor`)
        (`PrimitiveComponent.SetCollisionEnabled` _skelmeshcomp "PhysicsOnly")
        (`PrimitiveComponent.SetCollisionProfileName` _skelmeshcomp "BlockAll")
        (`PrimitiveComponent.SetSimulatePhysics` (`BaseWeaponClass.SkelMeshComp` _currentweapon) true)
        (`KismetSystemLibrary.Delay` 2.0)
        (`self.K2_DestroyActor` _currentweapon)))))

(fn `UserConstructionScript`
  (`parent.UserConstructionScript`))